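; TimeManager sequences the game's story steps, from loading screen and Louis's first phone call to the game-over screen.
; BeginPlay caches the SkyLight and Beast, and adds dynamic fog and VHS post-process materials to the player camera.
; StartStep events spawn the Beast and toggle deer, cabin and road steps on delays, with step 2 adding another call.
; Two ModifySky timelines animate fog and skylight between day and night colors.
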(event `self.ReceiveBeginPlay`
  (bind _returnvalue (`|CreateWidget` "/Game/Blueprint/Character/WDG_LoadingScreen.WDG_LoadingScreen_C"))
  (`UserWidget.AddToViewport` _returnvalue 0)
  (`KismetSystemLibrary.Delay` 3.0)
  (`Widget.RemoveFromParent` _returnvalue)
  (`|ExecutionSequence`
    (:`then_0`
      (bind _returnvalue_2 (`GameplayStatics.GetActorOfClass` "/Script/Engine.SkyLight"))
      (set `self.Post` _returnvalue_2)
      (bind _returnvalue_3 (`GameplayStatics.GetActorOfClass` "/Script/Engine.PostProcessVolume"))
      (set `self.PPvolume` _returnvalue_3)
      (bind _returnvalue_4 (`KismetMaterialLibrary.CreateDynamicMaterialInstance` "/Game/Materials/MI_Fog.MI_Fog"))
      (bind _output_get (set `self.PPMATFOG` _returnvalue_4))
      (bind _returnvalue_5 (`KismetMaterialLibrary.CreateDynamicMaterialInstance` "/Game/Materials/M_VHSEFFECT.M_VHSEFFECT"))
      (setmembers `PostProcessSettings` :`StructRef` (`CameraComponent.PostProcessSettings` (`self.GetComponentByClass` (`GameplayStatics.GetPlayerCharacter` 0) "/Script/Engine.CameraComponent")) :`WeightedBlendables` (make `WeightedBlendables` (`|MakeArray` (make `WeightedBlendable` 1.0 _output_get) (make `WeightedBlendable` 1.0 _returnvalue_5)))))
    (:`then_1`
      (`KismetSystemLibrary.Delay` 2.0)
      ;[1 1 1] Message vocal de louis
      (bind _asbp_chara_fps (cast `/Game/Blueprint/Character/BP_CharaFPS` (`GameplayStatics.GetPlayerCharacter` 0)))
      (`/Game/Blueprint/Character/BP_CharaFPS.PhoneCall` _asbp_chara_fps "/Game/Materials/Phone/MI_Phone_Louis.MI_Phone_Louis" "/Game/Sound/Louiscall.Louiscall" 12.0)
      (`KismetSystemLibrary.Delay` 10.0)
      (bind _returnvalue_6 (`GameplayStatics.GetActorOfClass` "/Game/Blueprint/SpawnableDeer.SpawnableDeer_C"))
      (`/Engine/EditorBlueprintResources/StandardMacros.IsValid` _returnvalue_6
        (:`Is Valid`
          (set `/Game/Blueprint/SpawnableDeer.StepActive` true _returnvalue_6))))
    (:`then_2`
      (bind _returnvalue_7 (`GameplayStatics.GetActorOfClass` "/Game/Blueprint/Beast.Beast_C"))
      (set `self.AsBeast` _returnvalue_7))))

(event `StartStep2`
  (`/Game/Blueprint/Beast.SpawnCreature` (`self.AsBeast`))
  (`self.ModifySky` 0)
  (`KismetSystemLibrary.Delay` 5.0)
  ;[1 1 1] Phone call avec louis qui halete
  (bind _asbp_chara_fps (cast `/Game/Blueprint/Character/BP_CharaFPS` (`GameplayStatics.GetPlayerCharacter` 0)))
  (`/Game/Blueprint/Character/BP_CharaFPS.PhoneCall` _asbp_chara_fps "/Game/Materials/Phone/MI_Phone_Louis.MI_Phone_Louis" "/Game/Sound/MC_2_Cue.MC_2_Cue" 12.0)
  (bind _returnvalue (`GameplayStatics.GetActorOfClass` "/Game/Blueprint/DeerOnBranch.DeerOnBranch_C"))
  (`KismetSystemLibrary.Delay` 10.0)
  (set `/Game/Blueprint/DeerOnBranch.StepActive` true _returnvalue))

(event `StartStep3`
  (bind _returnvalue (`GameplayStatics.GetActorOfClass` "/Game/Blueprint/DeerOnBranch.DeerOnBranch_C"))
  (set `/Game/Blueprint/DeerOnBranch.StepActive` false _returnvalue)
  (`/Game/Blueprint/Beast.SpawnCreature` (`self.AsBeast`))
  (`KismetSystemLibrary.Delay` 30.0)
  (bind _returnvalue_2 (`GameplayStatics.GetActorOfClass` "/Game/Blueprint/BP_Cabin.BP_Cabin_C"))
  (set `/Game/Blueprint/BP_Cabin.StepActive` true _returnvalue_2))

(event `StartStep4`
  (bind _asbeast (`self.AsBeast`))
  (bind _returnvalue (`GameplayStatics.GetActorOfClass` "/Game/Blueprint/BP_Cabin.BP_Cabin_C"))
  (set `/Game/Blueprint/BP_Cabin.StepActive` true _returnvalue)
  (`/Game/Blueprint/Beast.SpawnCreature` _asbeast)
  (set `/Game/Blueprint/Beast.VitesseBeast` 40.0 _asbeast)
  (bind _returnvalue_2 (`GameplayStatics.GetActorOfClass` "/Game/Blueprint/BP_Road.BP_Road_C"))
  (set `/Game/Blueprint/BP_Road.StepActive` true _returnvalue_2))

(event `ModifySky`
  (params (Step :type Integer))
  (bind _ppmatfog (`self.PPMATFOG`))
  (bind _lightcomponent (`SkyLight.LightComponent` (`self.Post`)))
  (bind (_direction _fogintensity _fog_color _lightintensity _lightcolor) (`Timeline|Timeline`)
    (:`Update`
      (`MaterialInstanceDynamic.SetScalarParameterValue` _ppmatfog "FogDistance" (* _fogintensity 4000.0))
      (`MaterialInstanceDynamic.SetVectorParameterValue` _ppmatfog "Color" (make `LinearColor` _fog_color _fog_color _fog_color 1.0))
      (`SkyLightComponent.SetIntensity` _lightcomponent _lightintensity)
      (`SkyLightComponent.SetLightColor` _lightcomponent (`KismetMathLibrary.LinearColorLerp` (`KismetMathLibrary.Conv_ColorToLinearColor` (`self.DayColor`)) (`KismetMathLibrary.Conv_ColorToLinearColor` (`self.Nightcolor`)) _lightcolor)))))

(event `GameOver`
  (bind _returnvalue (`|CreateWidget` "/Game/Blueprint/GameOverIcon.GameOverIcon_C"))
  (`UserWidget.AddToViewport` _returnvalue 0)
  (set `PlayerController.bShowMouseCursor` true (`GameplayStatics.GetPlayerController` 0)))

(event `ModifySky2`
  (params (Step :type Integer))
  (bind _ppmatfog (`self.PPMATFOG`))
  (bind _lightcomponent (`SkyLight.LightComponent` (`self.Post`)))
  (bind (_direction _fogintensity _fog_color _lightintensity _lightcolor) (`Timeline|Timeline_0`)
    (:`Update`
      (`MaterialInstanceDynamic.SetScalarParameterValue` _ppmatfog "FogDistance" (* _fogintensity 4000.0))
      (`MaterialInstanceDynamic.SetVectorParameterValue` _ppmatfog "Color" (make `LinearColor` _fog_color _fog_color _fog_color 1.0))
      (`SkyLightComponent.SetIntensity` _lightcomponent _lightintensity)
      (`SkyLightComponent.SetLightColor` _lightcomponent (`KismetMathLibrary.LinearColorLerp` (`KismetMathLibrary.Conv_ColorToLinearColor` (`self.DayColor`)) (`KismetMathLibrary.Conv_ColorToLinearColor` (`self.Nightcolor`)) _lightcolor)))))

(fn `UserConstructionScript`)