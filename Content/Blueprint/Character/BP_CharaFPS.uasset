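; BP_CharaFPS is a first-person player character with Enhanced Input look, yaw-relative movement and stamina-limited sprinting.
; BeginPlay adds the movement mapping context, and sprint input switches max walk speed between sprint and walk values.
; DrainStamina and RegenStamina macros clamp stamina, feeding self-calling Delay events, with empty stamina forcing a stop to sprinting.
; Tick prints stamina for debugging, and an EndlessWorldComponent initialization call sits unconnected.
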(event `self.ReceiveBeginPlay`
  ;[1 1 1] Begin play
  (bind _asplayer_controller (cast `PlayerController` (`self.GetController`)))
  (bind _returnvalue (pcsubsystem `EnhancedInputLocalPlayerSubsystem` _asplayer_controller))
  (`/Engine/EditorBlueprintResources/StandardMacros.IsValid` _returnvalue
    (:`Is Valid`
      (`EnhancedInputSubsystemInterface.AddMappingContext` _returnvalue "/Game/Input/IMC_Movement.IMC_Movement" 0 (struct)))))

(event `EnhancedInput|/Game/Input/InputAction/IA_Look`
  (params (ActionValue :type "Vector2D Structure") (ElapsedSeconds :type "Float (double-precision)") (TriggeredSeconds :type "Float (double-precision)") (InputAction :type "InputAction Object Reference" :default "/Game/Input/InputAction/IA_Look.IA_Look"))
  ;[1 1 1] Mouse Look
  (:`Triggered`
    ;;[1 1 1] Left-right
    (`self.AddControllerYawInput` ActionValue_X)
    ;;[1 1 1] Up-Down
    (`self.AddControllerPitchInput` ActionValue_Y)))

(event `EnhancedInput|/Game/Input/InputAction/IA_Move`
  (params (ActionValue :type "Vector2D Structure") (ElapsedSeconds :type "Float (double-precision)") (TriggeredSeconds :type "Float (double-precision)") (InputAction :type "InputAction Object Reference" :default "/Game/Input/InputAction/IA_Move.IA_Move"))
  (bind (_returnvalue_roll _returnvalue_pitch _returnvalue_yaw) (`KismetMathLibrary.BreakRotator` (`self.GetControlRotation`)))
  (bind _returnvalue (`KismetMathLibrary.MakeRotator` _returnvalue_roll 0.0 _returnvalue_yaw))
  ;[1 1 1] Movement
  (:`Triggered`
    (`self.AddMovementInput` (`KismetMathLibrary.GetRightVector` _returnvalue) ActionValue_X)
    (`self.AddMovementInput` (`KismetMathLibrary.GetForwardVector` _returnvalue) ActionValue_Y)))

(event `EnhancedInput|/Game/Input/InputAction/IA_Sprint`
  (params (ActionValue :type Boolean) (ElapsedSeconds :type "Float (double-precision)") (TriggeredSeconds :type "Float (double-precision)") (InputAction :type "InputAction Object Reference" :default "/Game/Input/InputAction/IA_Sprint.IA_Sprint"))
  ;[1 1 1] Sprint
  (:`Triggered`
    (`self.Sprint`)
    (`self.DrainStam`))
  (:`Completed`
    (`self.StopSprinting`)
    (`self.RegainStam`)))

(event `DrainStam`
  ;[1 1 1] Stamina Drain / Regen
  (`self.DrainStamina`
    (:`true`
      (`KismetSystemLibrary.Delay` 0.1)
      (`self.DrainStam`))))

(event `RegainStam`
  ;[1 1 1] Stamina Drain / Regen
  (`self.RegenStamina`
    (:`else`
      (`KismetSystemLibrary.Delay` 0.1)
      (`self.RegainStam`))))

(event `self.ReceiveTick`
  (params (DeltaSeconds :type "Float (single-precision)"))
  (`KismetSystemLibrary.PrintString` (`KismetStringLibrary.Conv_DoubleToString` (`self.Stamina`))))

(fn `Sprint`
  (set `self.IsSprinting` true)
  (set `CharacterMovementComponent.MaxWalkSpeed` (`self.SprintSpeed`) (`self.CharacterMovement`)))

(fn `StopSprinting`
  (set `self.IsSprinting` false)
  (set `CharacterMovementComponent.MaxWalkSpeed` (`self.WalkSpeed`) (`self.CharacterMovement`)))

(fn `UserConstructionScript`)