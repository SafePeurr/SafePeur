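; Beast actor that ends the game when the player gets within its kill distance.
; Each Tick, it measures the distance from its JeDevienneFou component to the player character's mesh, then calls GameOver on the TimeManager once through a DoOnce.
; An unconnected branch would intensify the player camera's vignette as proximity increases inside a danger distance, but it never runs.
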(event `self.ReceiveTick`
  (params (DeltaSeconds :type "Float (single-precision)"))
  (if (> (`self.KillDistance`) (`KismetMathLibrary.Vector_Distance` (`SceneComponent.K2_GetComponentLocation` (`self.Je_devienne_fou`)) (`SceneComponent.K2_GetComponentLocation` (`Character.Mesh` (`GameplayStatics.GetPlayerCharacter` 0)))))
    (`/Engine/EditorBlueprintResources/StandardMacros.DoOnce` false
      (:`Completed`
        (bind _returnvalue (`GameplayStatics.GetActorOfClass` "/Game/Blueprint/TimeManager.TimeManager_C"))
        (`/Game/Blueprint/TimeManager.GameOver` _returnvalue)))))

(fn `UserConstructionScript`)