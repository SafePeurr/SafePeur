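; Deer-on-branch scare actor that keeps placing itself ahead of the player until the player comes close to it.
; While StepActive is set, a delayed Tick check calls SpawnMe to move the deer along the player mesh's forward vector at fixed height whenever it is beyond Distance.
; Coming within close range fires BP_SoundManager's deer-sighting event once.
; A sphere-overlap pass that destroys nearby actors is left unconnected.
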(event `SpawnMe`
  (bind _mesh (`Character.Mesh` (`GameplayStatics.GetPlayerCharacter` 0)))
  (bind (_returnvalue_x _returnvalue_y) (`KismetMathLibrary.BreakVector` (+ (* (`SceneComponent.GetForwardVector` _mesh) (`self.Distance`)) (`SceneComponent.K2_GetComponentLocation` _mesh))))
  (`self.K2_SetActorLocation` (`KismetMathLibrary.MakeVector` _returnvalue_x _returnvalue_y 80.0) true))

(event `self.ReceiveTick`
  (params (DeltaSeconds :type "Float (single-precision)"))
  (bind _returnvalue (`KismetMathLibrary.Vector_Distance` (`SceneComponent.K2_GetComponentLocation` (`Actor.RootComponent` (`GameplayStatics.GetPlayerCharacter` 0))) (`SceneComponent.K2_GetComponentLocation` (`self.deerv1`))))
  (if (`self.StepActive`)
    (`KismetSystemLibrary.Delay` 1.0)
    (`KismetSystemLibrary.PrintString` "Lookingfortree")
    (if true
      (if (> _returnvalue (`self.Distance`))
        (`KismetSystemLibrary.PrintString` "Player didnt find der")
        (`self.SpawnMe`)
        (elif (> 500.0 _returnvalue)
          (`/Engine/EditorBlueprintResources/StandardMacros.DoOnce` false
            (:`Completed`
              (bind _returnvalue_2 (`GameplayStatics.GetActorOfClass` "/Game/Blueprint/BP_SoundManager.BP_SoundManager_C"))
              (`/Game/Blueprint/BP_SoundManager.Playerseedeeronbranch` _returnvalue_2)
              (`KismetSystemLibrary.PrintString` "Omg noo a deer :("))))))))

(fn `UserConstructionScript`)