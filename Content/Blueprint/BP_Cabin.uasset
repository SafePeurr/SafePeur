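; BP_Cabin is the cabin for a story step in which the player discovers a dead friend.
; While StepActive, a delayed Tick check respawns the cabin ahead of the player's mesh whenever it is beyond Distance, destroying overlapping actors around it.
; Nearing ManDeadActor fires once, playing a SoundManager reaction, clearing the Beast's timer and starting TimeManager step 4.
; A second delayed Tick branch repeats a creature sound at the body.
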(event `SpawnMe`
  (bind _mesh (`Character.Mesh` (`GameplayStatics.GetPlayerCharacter` 0)))
  (bind (_returnvalue_x _returnvalue_y) (`KismetMathLibrary.BreakVector` (+ (* (`SceneComponent.GetForwardVector` _mesh) (`self.Distance`)) (`SceneComponent.K2_GetComponentLocation` _mesh))))
  (`self.K2_SetActorLocation` (`KismetMathLibrary.MakeVector` _returnvalue_x _returnvalue_y 80.0) true)
  (bind _outactors (`KismetSystemLibrary.SphereOverlapActors` (`SceneComponent.K2_GetComponentLocation` (`self.cabin`)) 1000.0 (`self.Object Types`)))
  (for _array_element _outactors
    (`self.K2_DestroyActor` _array_element)))

(event `self.ReceiveTick`
  (params (DeltaSeconds :type "Float (single-precision)"))
  (`|ExecutionSequence`
    (:`then_0`
      (if (`self.StepActive`)
        (`KismetSystemLibrary.Delay` 1.0)
        (if (> (`KismetMathLibrary.Vector_Distance` (`SceneComponent.K2_GetComponentLocation` (`Character.Mesh` (`GameplayStatics.GetPlayerCharacter` 0))) (`SceneComponent.K2_GetComponentLocation` (`self.cabin`))) (`self.Distance`))
          (`KismetSystemLibrary.PrintString` "Cabin didnt found")
          (`self.SpawnMe`)
          (elif (> 250.0 (`KismetMathLibrary.Vector_Distance` (`SceneComponent.K2_GetComponentLocation` (`Character.Mesh` (`GameplayStatics.GetPlayerCharacter` 0))) (`SceneComponent.K2_GetComponentLocation` (`self.Man_Dead_Actor`))))
            (`/Engine/EditorBlueprintResources/StandardMacros.DoOnce` false
              (:`Completed`
                (bind _returnvalue (`GameplayStatics.GetActorOfClass` "/Game/Blueprint/BP_SoundManager.BP_SoundManager_C"))
                (`/Game/Blueprint/BP_SoundManager.Playerseedeeronbranch` _returnvalue)
                (`KismetSystemLibrary.PrintString` "OMG no my friend")
                (bind _returnvalue_2 (`GameplayStatics.GetActorOfClass` "/Game/Blueprint/Beast.Beast_C"))
                (`/Game/Blueprint/Beast.ClearTimer` _returnvalue_2)
                (bind _returnvalue_3 (`GameplayStatics.GetActorOfClass` "/Game/Blueprint/TimeManager.TimeManager_C"))
                (`/Game/Blueprint/TimeManager.StartStep4` _returnvalue_3)))))))
    (:`then_1`
      (if (`self.StepActive`)
        (`KismetSystemLibrary.Delay` 10.0)
        ;[1 1 1] HELP SOUNDS
        (`GameplayStatics.PlaySoundAtLocation` "/Game/Sound/SFX/creature/Close/SFX_creature_13.SFX_creature_13" (`SceneComponent.K2_GetComponentLocation` (`self.Man_Dead_Actor`)) (struct) 50.0 1.0 0.0 (`self.Attenuation Settings`) null null null)))))

(fn `UserConstructionScript`)