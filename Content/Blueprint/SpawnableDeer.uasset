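; Scripted deer encounter that freezes the player nearby and, once the deer dies, advances the game to step two.
; While active, a delayed Tick check moves it ahead of the player when farther than Distance, or disables player movement once within range.
; Die ragdolls the mesh via physics, cues BP_SoundManager, restores movement, calls TimeManager's StartStep2 and destroys the actor.
; Its box also destroys it on overlapping a StaticMeshActor.
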(event `SpawnMe`
  (bind _mesh (`Character.Mesh` (`GameplayStatics.GetPlayerCharacter` 0)))
  (bind (_returnvalue_x _returnvalue_y) (`KismetMathLibrary.BreakVector` (+ (* (`SceneComponent.GetForwardVector` _mesh) (`self.Distance`)) (`SceneComponent.K2_GetComponentLocation` _mesh))))
  (`self.K2_SetActorLocation` (`KismetMathLibrary.MakeVector` _returnvalue_x _returnvalue_y 80.0) true))

(event `self.ReceiveTick`
  (params (DeltaSeconds :type "Float (single-precision)"))
  (bind _returnvalue (`KismetMathLibrary.Vector_Distance` (`SceneComponent.K2_GetComponentLocation` (`Character.Mesh` (`GameplayStatics.GetPlayerCharacter` 0))) (`SceneComponent.K2_GetComponentLocation` (`self.deerv1`))))
  (if (`self.StepActive`)
    (`KismetSystemLibrary.Delay` 1.0)
    (if (> _returnvalue (`self.Distance`))
      (`KismetSystemLibrary.PrintString` "Player didnt find der")
      (`self.SpawnMe`)
      (elif (> 2000.0 _returnvalue)
        (`/Engine/EditorBlueprintResources/StandardMacros.DoOnce` false
          (:`Completed`
            (bind _asbp_chara_fps (cast `/Game/Blueprint/Character/BP_CharaFPS` (`GameplayStatics.GetPlayerCharacter` 0)))
            (`/Game/Blueprint/Character/BP_CharaFPS.DisablePlayerMovement` _asbp_chara_fps)))))))

(event `Die`
  (bind _returnvalue (`GameplayStatics.GetActorOfClass` "/Game/Blueprint/BP_SoundManager.BP_SoundManager_C"))
  (`/Game/Blueprint/BP_SoundManager.BirdGone` _returnvalue)
  (`PrimitiveComponent.SetSimulatePhysics` (`self.deerv1`) true)
  (bind _asbp_chara_fps (cast `/Game/Blueprint/Character/BP_CharaFPS` (`GameplayStatics.GetPlayerCharacter` 0)))
  (set `self.StepActive` false)
  ;[1 0.7727 0 1 60] ICI AJOUTER LA MAIN QUI ATTRAPE
  (`KismetSystemLibrary.Delay` 2.0)
  (bind _returnvalue_2 (`GameplayStatics.GetActorOfClass` "/Game/Blueprint/BP_SoundManager.BP_SoundManager_C"))
  (`/Game/Blueprint/BP_SoundManager.Player Deer dragged sound` _returnvalue_2)
  (`KismetSystemLibrary.Delay` 5.0)
  (`/Game/Blueprint/Character/BP_CharaFPS.EnablePlayerMovement` _asbp_chara_fps)
  (bind _returnvalue_3 (`GameplayStatics.GetActorOfClass` "/Game/Blueprint/TimeManager.TimeManager_C"))
  (`/Game/Blueprint/TimeManager.StartStep2` _returnvalue_3)
  (`self.K2_DestroyActor`))

(event `self.Box.OnComponentBeginOverlap`
  (params (OverlappedComponent :type "PrimitiveComponent Object Reference") (OtherActor :type "Actor Object Reference") (OtherComp :type "PrimitiveComponent Object Reference") (OtherBodyIndex :type Integer) (bFromSweep :type Boolean) (SweepResult :type "HitResult Structure (by ref)"))
  (cast `StaticMeshActor` OtherActor)
  (`self.K2_DestroyActor`))

(fn `UserConstructionScript`)