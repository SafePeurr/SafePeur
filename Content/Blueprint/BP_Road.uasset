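; BP_Road is a road actor with a car that relocates ahead of the player and ends the game when the player reaches the car.
; SpawnMe moves it along the player mesh's forward vector at fixed height, turns it crosswise, and destroys overlapped actors around the car.
; While StepActive, a delayed Tick check calls SpawnMe if the car is too far, or, when close, triggers BP_SoundManager and TimeManager's GameOver once.
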(event `SpawnMe`
  (bind _object_types (`self.Object Types`))
  (bind _returnvalue (`SceneComponent.K2_GetComponentLocation` (`self.car`)))
  (bind _mesh (`Character.Mesh` (`GameplayStatics.GetPlayerCharacter` 0)))
  (bind (_returnvalue_roll _returnvalue_pitch _returnvalue_yaw) (`KismetMathLibrary.BreakRotator` (`SceneComponent.K2_GetComponentRotation` _mesh)))
  (bind (_returnvalue_x _returnvalue_y) (`KismetMathLibrary.BreakVector` (+ (* (`SceneComponent.GetForwardVector` _mesh) (`self.Distance`)) (`SceneComponent.K2_GetComponentLocation` _mesh))))
  (`self.K2_SetActorLocationAndRotation` (`KismetMathLibrary.MakeVector` _returnvalue_x _returnvalue_y 80.0) (`KismetMathLibrary.MakeRotator` 0.0 0.0 (+ _returnvalue_yaw 90.0)))
  (bind _outactors (`KismetSystemLibrary.SphereOverlapActors` _returnvalue 1000.0 _object_types))
  (`KismetSystemLibrary.BoxOverlapActors` _returnvalue (100.0 100.0 100.0) _object_types)
  (for _array_element _outactors
    (`self.K2_DestroyActor` _array_element)))

(event `self.ReceiveTick`
  (params (DeltaSeconds :type "Float (single-precision)"))
  (`|ExecutionSequence`
    (:`then_0`
      (if (`self.StepActive`)
        (`KismetSystemLibrary.Delay` 1.0)
        (if (> (`KismetMathLibrary.Vector_Distance` (`SceneComponent.K2_GetComponentLocation` (`Character.Mesh` (`GameplayStatics.GetPlayerCharacter` 0))) (`SceneComponent.K2_GetComponentLocation` (`self.car`))) (* (`self.Distance`) 1.5))
          (`KismetSystemLibrary.PrintString` "Road not found")
          (`self.SpawnMe`)
          (elif (> 250.0 (`KismetMathLibrary.Vector_Distance` (`SceneComponent.K2_GetComponentLocation` (`Character.Mesh` (`GameplayStatics.GetPlayerCharacter` 0))) (`SceneComponent.K2_GetComponentLocation` (`self.car`))))
            (`/Engine/EditorBlueprintResources/StandardMacros.DoOnce` false
              (:`Completed`
                (bind _returnvalue (`GameplayStatics.GetActorOfClass` "/Game/Blueprint/BP_SoundManager.BP_SoundManager_C"))
                (`/Game/Blueprint/BP_SoundManager.Playerseedeeronbranch` _returnvalue)
                (bind _returnvalue_2 (`GameplayStatics.GetActorOfClass` "/Game/Blueprint/TimeManager.TimeManager_C"))
                (`/Game/Blueprint/TimeManager.GameOver` _returnvalue_2)))))))))

(fn `UserConstructionScript`)