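; Sound manager Blueprint that plays the game's player voice lines, forest ambience, gun and movement sounds through custom events.
; BeginPlay starts a happy-birds ambience, which BirdGone swaps for a quieter, lower-pitched horror loop.
; Effects play at the player's location, with gunshots picked randomly, though the fourth variant is never selected.
; Volumes multiply master by category settings, except cloth sounds, which are unscaled.
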(event `Playerseedeeronbranch`
  ;[1 1 1] Voix joueur
  (`GameplayStatics.PlaySound2D` "/Game/Sound/MC_3.MC_3" (* (`self.MasterVolume`) (`self.VoiceVolume`)) 1.0 0.0 null null))

(event `Player Deer dragged sound`
  ;[1 1 1] Voix joueur
  (`GameplayStatics.PlaySound2D` "/Game/Sound/MC_1.MC_1" (* (`self.MasterVolume`) (`self.VoiceVolume`)) 1.0 0.0 null null))

(event `self.ReceiveBeginPlay`
  ;[1 1 1] Ambiant music
  (bind _returnvalue (`GameplayStatics.SpawnSound2D` "/Game/Sound/SFX/AMB_forest_happy_birds.AMB_forest_happy_birds" (* (`self.MasterVolume`) (`self.AmbiantSoundVolume`)) 1.0 0.0 null))
  (set `self.Ambiantsound` _returnvalue))

(event `BirdGone`
  ;[1 1 1] Ambiant music
  (`AudioComponent.Stop` (`self.Ambiantsound`))
  (bind _returnvalue (`GameplayStatics.SpawnSound2D` "/Game/Sound/SFX/AMB_forest_horror.AMB_forest_horror" (* (* (`self.MasterVolume`) (`self.AmbiantSoundVolume`)) 0.5) 0.8 0.0 null))
  (set `self.Ambiantsound` _returnvalue))

(event `ReloadGun`
  ;[1 1 1] Shoot reload
  (`GameplayStatics.PlaySoundAtLocation` "/Game/Sound/SFX/Gun_reload.Gun_reload" (`self.K2_GetActorLocation` (`GameplayStatics.GetPlayerCharacter` 0)) (struct) (* (`self.MasterVolume`) (`self.FXVolume`)) 1.0 0.0 null null null null))

(event `Shoot`
  ;[1 1 1] Shoot reload
  (`GameplayStatics.PlaySoundAtLocation` (select `int` (`KismetMathLibrary.RandomInteger` 3) :`0` "/Game/Sound/SFX/Gun_shoot/Gun_shoot_01.Gun_shoot_01" :`1` "/Game/Sound/SFX/Gun_shoot/Gun_shoot_02.Gun_shoot_02" :`2` "/Game/Sound/SFX/Gun_shoot/Gun_shoot_03.Gun_shoot_03" :`3` "/Game/Sound/SFX/Gun_shoot/Gun_shoot_04.Gun_shoot_04" :!type "SoundBase Object Reference") (`self.K2_GetActorLocation` (`GameplayStatics.GetPlayerCharacter` 0)) (struct) (* (`self.MasterVolume`) (`self.FXVolume`)) 1.0 0.0 null null null null))

(event `RunStep`
  ;[1 1 1] Walking effects
  (`GameplayStatics.PlaySoundAtLocation` "/Game/Sound/SFX/Footsteps_player_run/RUN_Cue.RUN_Cue" (`self.K2_GetActorLocation` (`GameplayStatics.GetPlayerCharacter` 0)) (struct) (* (`self.MasterVolume`) (`self.FXVolume`)) 1.0 0.0 null null null null))

(event `Walkstep`
  ;[1 1 1] Walking effects
  (`GameplayStatics.PlaySoundAtLocation` "/Game/Sound/SFX/Footsteps_player_walk/FS_walk_08_Cue.FS_walk_08_Cue" (`self.K2_GetActorLocation` (`GameplayStatics.GetPlayerCharacter` 0)) (struct) (* (`self.MasterVolume`) (`self.FXVolume`)) 1.0 0.0 null null null null))

(event `ClothSound`
  ;[1 1 1] Walking effects
  (`GameplayStatics.PlaySoundAtLocation` "/Game/Sound/SFX/Footsteps_player_clothes/CUE_Clothes.CUE_Clothes" (`self.K2_GetActorLocation` (`GameplayStatics.GetPlayerCharacter` 0)) (struct) 1.0 1.0 0.0 null null null null))

(fn `UserConstructionScript`)